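; Player controller for the character select screen that keeps the player's view on a level cine camera.
; BeginPlay caches the first actor tagged CineCamera, and Tick restores it as the view target whenever the current target differs.
; Pressing F6 calls RequestImmediateStartGame to request an immediate game start.
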(event EventTick
  (params (DeltaSeconds :type Float%20%28single-precision%29))
  (Utilities|IsValid (Variables|Default|GetCineCamera)
    (:Is%20Valid
      (if (not (== (Pawn|GetViewTarget) (Variables|Default|GetCineCamera)))
        (Game|Player|SetViewTargetwithBlend (Variables|Default|GetCineCamera) 0.0 "VTBlend_Linear" 0.0 false)))))

(event EventBeginPlay
  (bind _outactors (Actor|GetAllActorswithTag "CineCamera"))
  (Utilities|IsValid (Utilities|Array|Get(acopy) _outactors)
    (:Is%20Valid
      (Variables|Default|SetCineCamera (Utilities|Array|Get(acopy) _outactors)))))

(event Input|KeyboardEvents|F6
  (params (Key :type Key%20Structure :default "None"))
  (:Pressed
    (Class|SMCharacterSelectPlayerController|RequestImmediateStartGame)))

(fn ConstructionScript)