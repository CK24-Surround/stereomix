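; BP_AICharacter is an AI character that follows and faces the first player character.
; Every tick it snaps its full rotation toward the player's location.
; From BeginPlay, ChasePlayer issues AI MoveTo with a wide acceptance radius and re-calls itself after a delay on success, or while no valid player exists.
; A failed move has no retry, so the chase loop ends there.
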(event Custom|Chase%20Player
  (if (Utilities|IsValid (Game|GetPlayerCharacter 0))
    (AI|AIMoveTo self "0, 0, 0" (Game|GetPlayerCharacter 0) 5e+02 false
      (:OnSuccess
        (Utilities|FlowControl|Delay 2.0)
        (CallFunction|ChasePlayer)))
    (else
      (Utilities|FlowControl|Delay 1.0)
      (CallFunction|ChasePlayer))))

(event EventBeginPlay
  (CallFunction|ChasePlayer))

(event Collision|EventActorBeginOverlap
  (params (OtherActor :type Actor%20Object%20Reference)))

(event EventTick
  (params (DeltaSeconds :type Float%20%28single-precision%29))
  (if (Utilities|IsValid (Game|GetPlayerCharacter 0))
    (Transformation|SetActorRotation (Math|Rotator|MakeRotfromX (- (Transformation|GetActorLocation (Game|GetPlayerCharacter 0)) (Transformation|GetActorLocation))))))

(fn ConstructionScript)