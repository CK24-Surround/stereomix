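; Base Blueprint for character previews that drives dissolve and animated eye material effects on the character mesh.
; The construction script creates a dynamic material instance per slot and keeps the "Eyes" one separately.
; NotifyDissolve runs a double-speed timeline into "Dissolve" on a hardcoded slot range, skipping a few indices.
; PlayTImeline sweeps the eye "Play" parameter between two frame values, scaling timeline rate to about 30 fps.
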(event Custom|NotifyDissolve
  (bind _eyetrack (Timeline|DissolveTimeline Play)
    (:Update
      (Components|Timeline|SetPlayRate (Variables|Default|GetDissolveTimeline) 2.0)
      (for _index (range 0 13)
        (if (!= _index 5)
          (if (!= _index 10)
            (if (!= _index 11)
              (Rendering|Material|SetScalarParameterValue (Utilities|Array|Get(acopy) (Variables|Default|GetMaterialArray) _index) "Dissolve" _eyetrack :!class /Script/Engine.MaterialInstanceDynamic)
              (Rendering|Material|SetMaterial (Variables|Default|GetCharacterMeshComponent) _index (Utilities|Array|Get(acopy) (Variables|Default|GetMaterialArray) _index)))))))))

(event Custom|PlayTImeline
  (params (Input :type Float%20%28double-precision%29) (Output :type Float%20%28double-precision%29))
  (bind _returnvalue (- Output Input))
  (bind _returnvalue_2 (* _returnvalue 0.03333))
  (Utilities|String|LogString (Utilities|String|ToString(Float) Input))
  (bind _eyetrack (Timeline|EyeTimeline PlayFromStart)
    (:Update
      (if (not (Math|Float|NearlyEqual(Float) _returnvalue_2 0.0 1e-06))
        (Components|Timeline|SetPlayRate (Variables|Default|GetEyeTimeline) (/ 1.0 _returnvalue_2))
        (CallFunction|UpdateEyeParameter (+ (* _eyetrack _returnvalue) Input))))))

(fn ConstructionScript
  (bind _charactermeshcomponent (Variables|Default|GetCharacterMeshComponent))
  (bind _returnvalue (Components|SkeletalMesh|GetSkeletalMeshAsset _charactermeshcomponent))
  (|CallParentFunction)
  (Utilities|IsValid _returnvalue
    (:Is%20Valid
      (for (_array_element _array_index) (Variables|/Script/Engine.SkeletalMesh|GetMaterials _returnvalue)
        (bind _returnvalue_2 (Rendering|Material|CreateDynamicMaterialInstance (Variables|Default|GetCharacterMeshComponent) _array_index 0 "None" :!class /Script/Engine.PrimitiveComponent))
        (Utilities|Array|SetArrayElem (Variables|Default|GetMaterialArray) _array_index _returnvalue_2 true)
        (if (== (.MaterialSlotName (Utilities|Struct|BreakSkeletalMaterial _array_element)) "Eyes")
          (Variables|Default|SetDynamicEyeMaterial _returnvalue_2))))))

(fn UpdateEyeParameter
  (params (Play :type Float%20%28double-precision%29))
  (Rendering|Material|SetScalarParameterValue (Variables|Default|GetDynamicEyeMaterial) "Play" Play :!class /Script/Engine.MaterialInstanceDynamic)
  (Rendering|Material|SetMaterialbyName (Variables|Default|GetCharacterMeshComponent) "Eyes" (Variables|Default|GetDynamicEyeMaterial)))