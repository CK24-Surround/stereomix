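; Anim notify base that changes the eye material on character preview actors.
; When triggered, it casts the mesh owner to BP_Preview_Base and checks that its dynamic eye material is valid.
; It then passes a configurable parameter value to the owner's UpdateEyeParameter and prints debug strings.
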(fn ReceivedNotify
  (params (MeshComp :type Skeletal%20Mesh%20Component%20Object%20Reference) (Animation :type Anim%20Sequence%20Base%20Object%20Reference) (EventReference :type Anim%20Notify%20Event%20Reference%20Structure%20%28by%20ref%29))
  (bind _parametervaluetoset (Variables|Default|GetParameterValueToSet))
  (Development|PrintString "AnimNotify")
  (bind _asbp_preview_base (Utilities|Casting|CastToBP_Preview_Base (Components|GetOwner MeshComp)))
  (Utilities|IsValid (Variables|/Game/StereoMix/Blueprints/Characters/Preview/BP_Preview_Base.BP_Preview_Base_C|GetDynamicEyeMaterial _asbp_preview_base)
    (:Is%20Valid
      (Default|UpdateEyeParameter _asbp_preview_base _parametervaluetoset)
      (Development|PrintString (Utilities|String|Append "Set eye parameter to " (Utilities|String|ToString(Float) _parametervaluetoset)))
      (return true))))