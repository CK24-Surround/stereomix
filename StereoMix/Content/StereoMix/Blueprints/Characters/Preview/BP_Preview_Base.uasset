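; Base Blueprint for a character-select preview that shows a character mesh through a scene capture limited to that mesh.
; The mesh is set in the construction script and on BeginPlay, which also plays a non-looping animation.
; It binds to player 0's character-select PlayerState and replays the animation whenever the character type changes.
; A check for matching character type and team exists but is disconnected, so replay is unfiltered.
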(event Custom|CharacterTypeChanged
  (params (NewCharacterType :type ESMCharacterType%20Enum :default "None"))
  (Components|Animation|PlayAnimation (Variables|Default|GetSkeletalMesh) (Variables|Default|GetCharacterAnimSequence) false))

(event EventBeginPlay
  (Components|SkeletalMesh|SetSkeletalMeshAsset (Variables|Default|GetSkeletalMesh) (Variables|Default|GetCharacterMesh))
  (Components|Animation|PlayAnimation (Variables|Default|GetSkeletalMesh) (Variables|Default|GetCharacterAnimSequence) false)
  (Rendering|SceneCapture|ShowOnlyComponent (Variables|Default|GetSceneCaptureComponent2D) (Variables|Default|GetSkeletalMesh))
  (bind _assmcharacter_select_player_state (Utilities|Casting|CastToSMCharacterSelectPlayerState (Game|GetPlayerState 0)))
  (bind _output_get (Variables|Default|SetPlayerState _assmcharacter_select_player_state))
  (EventDispatchers|AssignCharacterTypeChangedEvent _output_get (delegate Custom|CharacterTypeChanged)))

(fn ConstructionScript
  (Components|SkeletalMesh|SetSkeletalMeshAsset (Variables|Default|GetSkeletalMesh) (Variables|Default|GetCharacterMesh))
  (Rendering|SceneCapture|ShowOnlyComponent (Variables|Default|GetSceneCaptureComponent2D) (Variables|Default|GetSkeletalMesh)))