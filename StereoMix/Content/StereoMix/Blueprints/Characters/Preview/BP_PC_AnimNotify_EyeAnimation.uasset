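; Anim notify that triggers eye animation on character preview actors, using its start and end frame values.
; On notify, it casts the mesh owner to BP_CharacterPreviewBase and checks that its dynamic eye material is valid.
; It then passes both frames to the character's timeline function and updates the eye parameter with the start frame.
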(fn ReceivedNotify
  (params (MeshComp :type Skeletal%20Mesh%20Component%20Object%20Reference) (Animation :type Anim%20Sequence%20Base%20Object%20Reference) (EventReference :type Anim%20Notify%20Event%20Reference%20Structure%20%28by%20ref%29))
  (bind _asbp_character_preview_base (Utilities|Casting|CastToBP_CharacterPreviewBase (Components|GetOwner MeshComp)))
  (Utilities|IsValid (Variables|/Game/StereoMix/Blueprints/Characters/Preview/BP_CharacterPreviewBase.BP_CharacterPreviewBase_C|GetDynamicEyeMaterial _asbp_character_preview_base)
    (:Is%20Valid
      (Default|PlayTImeline _asbp_character_preview_base (Variables|Default|GetStartFrame) (Variables|Default|GetEndFrame))
      (Default|UpdateEyeParameter _asbp_character_preview_base (Variables|Default|GetStartFrame))
      (return true))))