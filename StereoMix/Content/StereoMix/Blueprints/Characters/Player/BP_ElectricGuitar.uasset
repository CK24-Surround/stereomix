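; Electric guitar player character Blueprint that drives a randomly timed, looping eye blink.
; On BeginPlay it looks up its eye animation control component and starts blinking only if that component is valid.
; Each blink waits a random delay, then plays the Eye timeline, feeding its FlipRatio to the component every update and scheduling the next blink when finished.
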(event Custom|EyeBlink
  (Utilities|FlowControl|Delay (Math|Random|RandomFloatinRange 0.2 4.0))
  (bind _flipratio (Timeline|Eye PlayFromStart)
    (:Update
      (Default|UpdateEyeBlink (Variables|Default|GetEyeAnimationController) _flipratio))
    (:Finished
      (CallFunction|EyeBlink))))

(event EventBeginPlay
  (bind _output_get (Variables|Default|SetEyeAnimationController (Actor|GetComponentbyClass "/Game/StereoMix/Effects/Blueprints/BP_EyeAnimationControlComponent.BP_EyeAnimationControlComponent_C")))
  (Utilities|IsValid _output_get
    (:Is%20Valid
      (CallFunction|EyeBlink))))

(fn ConstructionScript)