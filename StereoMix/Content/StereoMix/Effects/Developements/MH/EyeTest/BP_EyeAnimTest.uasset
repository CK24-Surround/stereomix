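; Test Blueprint that animates random, repeating eye blinks on the SKEDMElec mesh.
; BeginPlay creates dynamic material instances for two eye material slots and starts the EyeBlink loop.
; After each random delay, the Eye timeline restarts and drives the "Play" scalar parameter on both instances.
; EyeBlink re-calls itself after the delay and when the timeline finishes.
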(event Custom|EyeBlink
  (Utilities|FlowControl|Delay (Math|Random|RandomFloatinRange 0.2 4.0))
  (CallFunction|EyeBlink)
  (bind _track_1 (Timeline|Eye PlayFromStart)
    (:Update
      (Rendering|Material|SetScalarParameterValue (stale EventBeginPlay _returnvalue) "Play" _track_1 :!class /Script/Engine.MaterialInstanceDynamic)
      (Rendering|Material|SetScalarParameterValue (stale EventBeginPlay _returnvalue_2) "Play" _track_1 :!class /Script/Engine.MaterialInstanceDynamic))
    (:Finished
      (CallFunction|EyeBlink))))

(event EventBeginPlay
  (bind _sk_edmelec (Variables|Default|GetSK_EDMElec))
  (bind _returnvalue (Rendering|Material|CreateDynamicMaterialInstance (Rendering|Material|GetMaterial _sk_edmelec 1) "Eye1" "None" :!class /Script/Engine.KismetMaterialLibrary))
  (Rendering|Material|SetMaterial (Variables|Default|GetSK_EDMElec) 1 _returnvalue)
  (bind _returnvalue_2 (Rendering|Material|CreateDynamicMaterialInstance (Rendering|Material|GetMaterial _sk_edmelec 3) "Eye2" "None" :!class /Script/Engine.KismetMaterialLibrary))
  (Rendering|Material|SetMaterial (Variables|Default|GetSK_EDMElec) 3 _returnvalue_2)
  (CallFunction|EyeBlink))

(fn ConstructionScript)