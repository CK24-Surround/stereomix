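; Actor component that drives eye blinking on a character's skeletal mesh through material parameters.
; On BeginPlay it finds the owner's SkeletalMeshComponent and creates dynamic material instances for the InEye and OutEye material slots.
; UpdateEyeBlink writes a given flip ratio to the same named scalar parameter on both instances, leaving blink timing to the caller.
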(event EventBeginPlay
  (bind _output_get (Variables|Default|SetOwnerMesh (Actor|GetComponentbyClass (Components|GetOwner) "/Script/Engine.SkeletalMeshComponent")))
  (Utilities|IsValid _output_get
    (:Is%20Valid
      (bind _mid (CallFunction|CreateandSetEyeMID (Variables|Default|GetInEyeMaterialIndex)))
      (Variables|Default|SetInEyeMID _mid)
      (bind _mid_2 (CallFunction|CreateandSetEyeMID (Variables|Default|GetOutEyeMaterialIndex)))
      (Variables|Default|SetOutEyeMID _mid_2))))

(fn CreateandSetEyeMID
  (params (InIndex :type Integer))
  (bind _output_get (LocalVariables|SetOriginalMaterial (Rendering|Material|GetMaterial (Variables|Default|GetOwnerMesh) InIndex)))
  (Utilities|IsValid _output_get
    (:Is%20Valid
      (bind _returnvalue (Rendering|Material|CreateDynamicMaterialInstance (Variables|Default|GetOwnerMesh) InIndex (LocalVariables|GetOriginalMaterial) "None" :!class /Script/Engine.PrimitiveComponent))
      (return _returnvalue))
    (:Is%20Not%20Valid
      (return 0))))

(fn UpdateEyeBlink
  (params (FlipRatio :type Float%20%28double-precision%29))
  (Utilities|FlowControl|Sequence
    (:then_0
      (bind _ineyemid (Variables|Default|GetInEyeMID)
        (:then
          (Rendering|Material|SetScalarParameterValue _ineyemid (Variables|Default|GetEyeParameterName) FlipRatio :!class /Script/Engine.MaterialInstanceDynamic))
        (:else)))
    (:then_1
      (bind _outeyemid (Variables|Default|GetOutEyeMID)
        (:then
          (Rendering|Material|SetScalarParameterValue _outeyemid (Variables|Default|GetEyeParameterName) FlipRatio :!class /Script/Engine.MaterialInstanceDynamic))
        (:else)))))